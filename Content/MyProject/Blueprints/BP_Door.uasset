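; BP_Door is an automatic door that swings open while any NPC is near and closes when none remain.
; Begin and end overlap events on the TriggerOpenDoor volume count NPCBase actors in NumOverlapNPCs.
; Tick polls that count, playing a timeline forward or in reverse to drive the Door component's relative yaw.
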(event `self.ReceiveTick`
  (params (DeltaSeconds :type "Float (single-precision)"))
  ;[1 1 1] Close door if no NPCs near, otherwise open it
  (if (> (`self.NumOverlapNPCs`) 0)
    (bind (_direction _newtrack_0) (`Timeline|Timeline_0` :!label _label)
      (:`Update`
        (`SceneComponent.K2_SetRelativeRotation` (`self.Door`) (`KismetMathLibrary.MakeRotator` 0.0 0.0 _newtrack_0) false false)))
    (else
      (goto _label :!via `Reverse`))))

(event `self.TriggerOpenDoor.OnComponentBeginOverlap`
  (params (OverlappedComponent :type "PrimitiveComponent Object Reference") (OtherActor :type "Actor Object Reference") (OtherComp :type "PrimitiveComponent Object Reference") (OtherBodyIndex :type Integer) (bFromSweep :type Boolean) (SweepResult :type "HitResult Structure (by ref)"))
  ;[1 1 1] Keep track of number of NPCs near door
  (cast `/Game/MyProject/Blueprints/NPCBase` OtherActor)
  (set `self.NumOverlapNPCs` (+ (`self.NumOverlapNPCs`) 1)))

(event `self.TriggerOpenDoor.OnComponentEndOverlap`
  (params (OverlappedComponent :type "PrimitiveComponent Object Reference") (OtherActor :type "Actor Object Reference") (OtherComp :type "PrimitiveComponent Object Reference") (OtherBodyIndex :type Integer))
  ;[1 1 1] Keep track of number of NPCs near door
  (cast `/Game/MyProject/Blueprints/NPCBase` OtherActor)
  (set `self.NumOverlapNPCs` (- (`self.NumOverlapNPCs`) 1)))

(fn `UserConstructionScript`)