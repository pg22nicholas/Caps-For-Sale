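; BP_HatManager is an actor that keeps a single BP_Hat spawned at its own transform, starting on BeginPlay.
; The Pickup input calls PickupHat on the current hat, clears the reference, and spawns a replacement after a delay.
; The ResetHat input destroys the current hat and respawns one after a shorter delay, without the validity check that Pickup uses.
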(event `self.ReceiveBeginPlay`
  (`self.SpawnNewHat`))

(event `InputAction|ResetHat`
  (params (Key :type "Key Structure"))
  ;[1 1 1] Reset the hat, deleting it and delaying until a new one spawns
  (:`Pressed`
    (`self.K2_DestroyActor` (`self.HatSpawned`))
    (`KismetSystemLibrary.Delay` 3.0)
    (`self.SpawnNewHat`)))

(event `InputAction|Pickup`
  (params (Key :type "Key Structure"))
  ;[1 1 1] Pickup the hat and delay spawning another
  (:`Pressed`
    (if (`KismetSystemLibrary.IsValid` (`self.HatSpawned`))
      (`/Game/MyProject/Blueprints/BP_Hat.PickupHat` (`self.HatSpawned`))
      (set `self.HatSpawned` null)
      (`KismetSystemLibrary.Delay` 7.0)
      (`self.SpawnNewHat`))))

(fn `SpawnNewHat`
  (bind _returnvalue (`|SpawnActorFromClass` "/Game/MyProject/Blueprints/BP_Hat.BP_Hat_C" (`self.GetTransform`) "Undefined" "OverrideRootScale" null null))
  (set `self.HatSpawned` _returnvalue))

(fn `UserConstructionScript`)