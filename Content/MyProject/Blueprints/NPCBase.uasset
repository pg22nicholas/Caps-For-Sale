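; NPC customer character that wanders to random reachable points and wants one randomly chosen hat color, shown by its ground marker.
; BuyHat accepts only that color, attaches the hat and makes the NPC ascend until destroyed.
; A random timer flags it as exploding, so a hatless NPC swells, pops and notifies ThirdPersonGameMode.
; Tick drives all three states, and BeginPlay spawns an AI controller so dynamically spawned NPCs can move.
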(event `self.ReceiveBeginPlay`
  (`|ExecutionSequence`
    (:`then_0`
      ;[1 1 1] Allows dynamically spawned NPC to use AiMoveTo
      (`self.SpawnDefaultController`)
      (`Controller.Possess` (`self.GetController`) self))
    (:`then_1`
      ;[1 1 1] Set the type of hat color the NPC will buy
      (bind _output_get (set `self.NPCHatColorCanBuy` (cast `/Game/MyProject/HatColors` (`KismetMathLibrary.Conv_Int64ToByte` (`KismetMathLibrary.RandomInteger64InRange` 0 2)))))
      (`PrimitiveComponent.SetMaterial` (`self.GroundColorMarker`) 0 (`|GetArrayItem` (`self.ColorMaterialsRelatedToHat`) (`KismetMathLibrary.Conv_ByteToInt` _output_get))))
    (:`then_2`
      ;[1 1 1] After a delay, set NPC to exploding
      (`KismetSystemLibrary.Delay` (`KismetMathLibrary.RandomFloatInRange` 20.0 25.0))
      (set `self.bExploding` true))))

(event `self.ReceiveTick`
  (params (DeltaSeconds :type "Float (single-precision)"))
  (bind _returnvalue (`GameplayStatics.GetWorldDeltaSeconds`))
  (bind _returnvalue_2 (`GameplayStatics.GetWorldDeltaSeconds`))
  (if (`self.bBoughtHat`)
    (`MovementComponent.StopMovementImmediately` (`self.CharacterMovement`))
    (if (> (`self.TimeSinceStartAscending`) 5.0)
      (`self.DestroyNPC`)
      (else
        ;[1 1 1] NPC ascends into sky for a time after buying a hat
        (`SceneComponent.K2_SetWorldLocation` (`self.Mesh`) (+ (`SceneComponent.K2_GetComponentLocation` (`self.Mesh`)) (* (`self.AscendSpeed`) _returnvalue)) false false)
        (set `self.TimeSinceStartAscending` (+ (`self.TimeSinceStartAscending`) _returnvalue))))
    (elif (`self.bExploding`)
      (`MovementComponent.StopMovementImmediately` (`self.CharacterMovement`))
      (if (> (`self.TimeSinceStartExploding`) 2.0)
        (`self.DestroyNPC`)
        (else
          ;[1 1 1] NPC expands for a time, exploding after some time
          (`SceneComponent.SetWorldScale3D` (`self.Mesh`) (+ (`SceneComponent.K2_GetComponentScale` (`self.Mesh`)) (* (`self.ExplodeSpeed`) _returnvalue_2)))
          (set `self.TimeSinceStartExploding` (+ (`self.TimeSinceStartExploding`) _returnvalue_2))))
      (else
        ;[1 1 1] Move NPC to random location after a delay
        (if (`self.bRecentlySpawned`)
          (set `self.bRecentlySpawned` false)
          (else
            (`KismetSystemLibrary.Delay` (`KismetMathLibrary.RandomFloatInRange` 6.0 9.0))))
        (set `self.bMoving` true)
        (`|AIMoveTo` self (`NavigationSystemV1.K2_GetRandomReachablePointInRadius` (`self.K2_GetActorLocation`) 3000.0 null null) null
          (:`then`
            _)
          (:`OnFail`
            _))
        (set `self.bMoving` false)))))

(fn `BuyHat`
  (params (HatForNpcToBuy :type "/Game/MyProject/Blueprints/BP_Hat Object Reference"))
  (returns (bBought :type Boolean))
  (bind _returnvalue (`|EnumEquality` (`/Game/MyProject/Blueprints/BP_Hat.HatColor` HatForNpcToBuy) (`self.NPCHatColorCanBuy`)))
  (if (`self.bBoughtHat`)
    (return false) ; NPC already has a hat
    (else
      ;[1 1 1] Check if valid hat color
      (if _returnvalue
        (if (`self.bExploding`)
          (return false) ; NPC is process of exploding
          (else
            ;[1 1 1] NPC buys valid hat
            (`KismetSystemLibrary.PrintString` "Valid color")
            (`self.K2_AttachToComponent` HatForNpcToBuy (`self.HatStartSpawn`) "None" "SnapToTarget" "SnapToTarget" "SnapToTarget" true)
            (set `self.HatOnHead` HatForNpcToBuy)
            (set `self.bBoughtHat` true)
            ;[1 1 1] Play heavently sound
            (`GameplayStatics.PlaySoundAtLocation` "/Game/MyProject/Sound/heavently_sound.heavently_sound" (`KismetMathLibrary.TransformLocation` (`self.GetTransform`)) (struct) 1.0 1.0 0.0 null null null)
            (return _returnvalue)))
        (else
          (return false) ; Invalid Hat Color
        )))))

(fn `DestroyNPC`
  (`|ExecutionSequence`
    (:`then_0`
      (if (`self.bExploding`)
        ;[1 1 1] Notify GameMode if NPC exploded
        (bind _asthird_person_game_mode (cast `/Game/ThirdPersonBP/Blueprints/ThirdPersonGameMode` (`GameplayStatics.GetGameMode`)))
        (`/Game/ThirdPersonBP/Blueprints/ThirdPersonGameMode.NPC exploded` _asthird_person_game_mode)
        ;[1 1 1] Play pop noise
        (`GameplayStatics.PlaySoundAtLocation` "/Game/MyProject/Sound/pop_sound.pop_sound" (`KismetMathLibrary.TransformLocation` (`self.GetTransform`)) (struct) 1.0 1.0 0.0 null null null)))
    (:`then_1`
      ;[1 1 1] Destroy NPC Character and play pop noise
      (`|ExecutionSequence`
        (:`then_0`
          (if (`KismetSystemLibrary.IsValid` (`self.HatOnHead`))
            (`self.K2_DestroyActor` (`self.HatOnHead`))))
        (:`then_1`
          (`self.K2_DestroyActor`))))))

(fn `UserConstructionScript`)