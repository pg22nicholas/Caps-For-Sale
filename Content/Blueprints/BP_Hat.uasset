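; BP_Hat is a hard hat that the player can pick up and wear.
; On BeginPlay it picks one of three HatColors enum values at random and applies the matching entry from HatColorMaterials to its mesh.
; PickupHat casts player 0's pawn to MyThirdPerson and passes itself to that character's AddHat, which handles the attachment.
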(event `self.ReceiveBeginPlay`
  ;[1 1 1] Make the hat a random color from a set of materials
  (bind _output_get (set `self.HatColor` (cast `/Game/Blueprints/HatColors` (`KismetMathLibrary.Conv_IntToByte` (`KismetMathLibrary.RandomInteger` 3)))))
  (`PrimitiveComponent.SetMaterial` (`self.SM_HardHat_01b`) 0 (`|GetArrayItem` (`self.HatColorMaterials`) (`KismetMathLibrary.Conv_ByteToInt` _output_get))))

(fn `PickupHat`
  ;[1 1 1] Player picks up hat and puts on head
  (bind _asmy_third_person (cast `/Game/Blueprints/MyThirdPerson` (`GameplayStatics.GetPlayerPawn` 0)))
  (`/Game/Blueprints/MyThirdPerson.AddHat` _asmy_third_person self))

(fn `UserConstructionScript`
  (`parent.UserConstructionScript`))