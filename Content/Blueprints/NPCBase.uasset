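; Base NPC character that wanders, can buy one hat of a randomly assigned color, and explodes after a delay.
; BeginPlay spawns an AI controller for runtime-spawned NPCs and colors a ground marker to show the wanted hat.
; Tick drives delayed random-point movement, then explosion by mesh growth, notifying ThirdPersonGameMode before destroying NPC and hat.
; BuyHat attaches a matching hat to the head, but buying never cancels the explosion.
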(event `self.ReceiveBeginPlay`
  (`|ExecutionSequence`
    (:`then_0`
      ;[1 1 1] Allows dynamically spawned NPC to use AiMoveTo
      (`self.SpawnDefaultController`)
      (`Controller.Possess` (`self.GetController`) self))
    (:`then_1`
      ;[1 1 1] Set the type of hat color the NPC will buy
      (bind _output_get (set `self.NPCHatColorCanBuy` (cast `/Game/Blueprints/HatColors` (`KismetMathLibrary.Conv_Int64ToByte` (`KismetMathLibrary.RandomInteger64InRange` 0 2)))))
      (`PrimitiveComponent.SetMaterial` (`self.GroundColorMarker`) 0 (`|GetArrayItem` (`self.ColorMaterialsRelatedToHat`) (`KismetMathLibrary.Conv_ByteToInt` _output_get))))
    (:`then_2`
      ;[1 1 1] After a delay, set NPC to exploding
      (`KismetSystemLibrary.Delay` (`KismetMathLibrary.RandomFloatInRange` 5.0 5.0))
      (set `self.bExploding` true))))

(event `self.ReceiveTick`
  (params (DeltaSeconds :type "Float (single-precision)"))
  (bind _returnvalue (`GameplayStatics.GetWorldDeltaSeconds`))
  (if (`self.bExploding`)
    (`MovementComponent.StopMovementImmediately` (`self.CharacterMovement`))
    (if (> (`self.TimeSinceStartExploding`) 2.0)
      (`self.DestroyNPC`)
      (else
        ;[1 1 1] Expand NPC to simulate exploding
        (`SceneComponent.SetWorldScale3D` (`self.Mesh`) (+ (`SceneComponent.K2_GetComponentScale` (`self.Mesh`)) (* (`self.ExplodeSpeed`) _returnvalue)))
        (set `self.TimeSinceStartExploding` (+ (`self.TimeSinceStartExploding`) _returnvalue))))
    (else
      ;[1 1 1] Move NPC to random location after a delay
      (`KismetSystemLibrary.Delay` (`KismetMathLibrary.RandomFloatInRange` 3.0 6.0))
      (set `self.bMoving` true)
      (`|AIMoveTo` self (`NavigationSystemV1.K2_GetRandomReachablePointInRadius` (`self.K2_GetActorLocation`) 1500.0 null null) null
        (:`then`
          _)
        (:`OnFail`
          _))
      (set `self.bMoving` false))))

(fn `BuyHat`
  (params (HatForNpcToBuy :type "/Game/Blueprints/BP_Hat Object Reference"))
  (returns (bBought :type Boolean))
  (bind _returnvalue (`|EnumEquality` (`/Game/Blueprints/BP_Hat.HatColor` HatForNpcToBuy) (`self.NPCHatColorCanBuy`)))
  (if (`self.bBoughtHat`)
    ;[1 1 1] NPC already has a hat
    (`KismetSystemLibrary.PrintString` "Already has a hat")
    (return false)
    (else
      ;[1 1 1] Check if valid hat color
      (if _returnvalue
        ;[1 1 1] NPC buys hat if it's proper color
        (`KismetSystemLibrary.PrintString` "Valid color")
        (`self.K2_AttachToComponent` HatForNpcToBuy (`self.HatStartSpawn`) "None" "SnapToTarget" "SnapToTarget" "SnapToTarget" true)
        (set `self.HatOnHead` HatForNpcToBuy)
        (set `self.bBoughtHat` true)
        (return _returnvalue)
        (else
          ;[1 1 1] Invalid hat color
          (`KismetSystemLibrary.PrintString` "Invalid color")
          (return false))))))

(fn `DestroyNPC`
  (`|ExecutionSequence`
    (:`then_0`
      ;[1 1 1] Notify GameMode NPC exploded
      (bind _asthird_person_game_mode (cast `/Game/ThirdPersonBP/Blueprints/ThirdPersonGameMode` (`GameplayStatics.GetGameMode`)))
      (`/Game/ThirdPersonBP/Blueprints/ThirdPersonGameMode.NPC exploded` _asthird_person_game_mode))
    (:`then_1`
      ;[1 1 1] Destroy NPC Character
      (`|ExecutionSequence`
        (:`then_0`
          (if (`KismetSystemLibrary.IsValid` (`self.HatOnHead`))
            (`self.K2_DestroyActor` (`self.HatOnHead`))))
        (:`then_1`
          (`self.K2_DestroyActor`))))))

(fn `UserConstructionScript`)