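; BP_HatManager is an actor that spawns a BP_Hat at its own transform on BeginPlay and keeps a reference to it.
; The ResetHat input destroys the current hat and respawns one after a short delay.
; The Pickup input calls PickupHat on the hat, releases the reference, and spawns a replacement after a longer delay.
; Both inputs use the stored reference without a validity check.
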(event `self.ReceiveBeginPlay`
  (`self.SpawnNewHat`))

(event `InputAction|ResetHat`
  (params (Key :type "Key Structure"))
  (:`Pressed`
    (`self.K2_DestroyActor` (`self.HatSpawned`))
    (`KismetSystemLibrary.Delay` 3.0)
    (`self.SpawnNewHat`)))

(event `InputAction|Pickup`
  (params (Key :type "Key Structure"))
  (:`Pressed`
    (`/Game/Blueprints/BP_Hat.PickupHat` (`self.HatSpawned`))
    (set `self.HatSpawned` null)
    (`KismetSystemLibrary.Delay` 7.0)
    (`self.SpawnNewHat`)))

(fn `SpawnNewHat`
  (bind _returnvalue (`|SpawnActorFromClass` "/Game/Blueprints/BP_Hat.BP_Hat_C" (`self.GetTransform`) "Undefined" "OverrideRootScale" null null))
  (set `self.HatSpawned` _returnvalue))

(fn `UserConstructionScript`)